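; BP_FRD is a test actor that moves until its world X reaches 100 and times how long that takes.
; BeginPlay records and prints the real-time start, then each Tick adds Velocity as a local offset without delta-time scaling, so speed depends on frame rate.
; On reaching the threshold, a DoOnce prints "Arrived" and the elapsed real time.
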(event `self.ReceiveBeginPlay`
  (bind _returnvalue (`GameplayStatics.GetRealTimeSeconds`))
  (`KismetSystemLibrary.PrintString` (`KismetStringLibrary.Conv_DoubleToString` _returnvalue))
  (set `self.BeginPlayTime` _returnvalue))

(event `self.ReceiveTick`
  (params (DeltaSeconds :type "Float (single-precision)"))
  (bind _returnvalue_x (`KismetMathLibrary.BreakVector` (`self.K2_GetActorLocation`)))
  (if (>= _returnvalue_x 100.0)
    (`/Engine/EditorBlueprintResources/StandardMacros.DoOnce` false
      (:`Completed`
        (`KismetSystemLibrary.PrintString` "Arrived")
        (set `self.FinishPlayTime` (`GameplayStatics.GetRealTimeSeconds`))
        (`KismetSystemLibrary.PrintString` (`KismetStringLibrary.Conv_DoubleToString` (- (`self.FinishPlayTime`) (`self.BeginPlayTime`))))))
    (else
      (`self.K2_AddActorLocalOffset` (`self.Velocity`)))))

(fn `UserConstructionScript`)